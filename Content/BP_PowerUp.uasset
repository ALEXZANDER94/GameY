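; Pickup actor that grants the player a damage, range, health or speed upgrade, chosen by its Effect.
; Overlap on PickUpArea only tracks whether the player is in range; PowerUpPickedUp, not called within this file, triggers the pickup.
; ApplyPowerUp hides the actor, raises the matching character stat (LifeSpan for range, health also refills) and increments that type's GameMode counter.
; The actor destroys itself after a short delay.
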(event Custom|PowerUpPickedUp
  (params (DestroyedActor :type Actor%20Object%20Reference))
  (CallFunction|ApplyPowerUp (Variables|Default|GetEffect))
  (Utilities|FlowControl|Delay 1.5)
  (Actor|DestroyActor))

(event Custom|PlayerEntersPickupArea
  (params (OverlappedComponent :type Primitive%20Component%20Object%20Reference) (OtherActor :type Actor%20Object%20Reference) (OtherComp :type Primitive%20Component%20Object%20Reference) (OtherBodyIndex :type Integer) (bFromSweep :type Boolean) (SweepResult :type Hit%20Result%20Structure%20%28by%20ref%29))
  (if (== OtherActor (Game|Player|GetPlayerPawn 0))
    (Variables|Default|SetPlayerInRangeOfPowerUp true)))

(event Custom|PlayerLeavesPickupArea
  (params (OverlappedComponent :type Primitive%20Component%20Object%20Reference) (OtherActor :type Actor%20Object%20Reference) (OtherComp :type Primitive%20Component%20Object%20Reference) (OtherBodyIndex :type Integer))
  (if (== OtherActor (Game|Player|GetPlayerPawn 0))
    (Variables|Default|SetPlayerInRangeOfPowerUp false)))

(event EventBeginPlay
  (Collision|AssignOnComponentBeginOverlap (Variables|Default|GetPickUpArea) (delegate Custom|PlayerEntersPickupArea))
  (Collision|AssignOnComponentEndOverlap (Variables|Default|GetPickUpArea) (delegate Custom|PlayerLeavesPickupArea)))

(event Collision|EventActorBeginOverlap
  (params (OtherActor :type Actor%20Object%20Reference)))

(event EventTick
  (params (DeltaSeconds :type Float%20%28single-precision%29)))

(fn ConstructionScript)

(fn ApplyPowerUp
  (params (PowerUpEffect :type Byte) (Instigator :type First%20Person%20Projectile%20Object%20Reference))
  (Rendering|SetActorHiddenInGame true)
  (Variables|Default|SetIsDestroyed true)
  (switch Utilities|FlowControl|Switch|SwitchonEffectType (Utilities|Enum|ByteToEnumEffectType PowerUpEffect)
    (:Damage
      (bind _asfirst_person_character (Utilities|Casting|CastToFirstPersonCharacter (Game|Player|GetPlayerPawn 0)))
      (Variables|/Game/FirstPersonBP/Blueprints/FirstPersonCharacter.FirstPersonCharacter_C|SetDamage _asfirst_person_character (+ (Variables|/Game/FirstPersonBP/Blueprints/FirstPersonCharacter.FirstPersonCharacter_C|GetDamage _asfirst_person_character) 25.0))
      (bind _asfirst_person_game_mode (Utilities|Casting|CastToFirstPersonGameMode (Game|GetGameMode)))
      (Math|Integer|IncrementInt (Variables|/Game/FirstPersonBP/Blueprints/FirstPersonGameMode.FirstPersonGameMode_C|GetDmgPickupCount _asfirst_person_game_mode)
        (:%20%20
          (Variables|Default|SetIsDestroyed true))))
    (:Range
      (bind _asfirst_person_character_2 (Utilities|Casting|CastToFirstPersonCharacter (Game|Player|GetPlayerPawn 0)))
      (Variables|/Game/FirstPersonBP/Blueprints/FirstPersonCharacter.FirstPersonCharacter_C|SetLifeSpan _asfirst_person_character_2 (+ (Variables|/Game/FirstPersonBP/Blueprints/FirstPersonCharacter.FirstPersonCharacter_C|GetLifeSpan _asfirst_person_character_2) 0.1))
      (bind _asfirst_person_game_mode_2 (Utilities|Casting|CastToFirstPersonGameMode (Game|GetGameMode)))
      (Math|Integer|IncrementInt (Variables|/Game/FirstPersonBP/Blueprints/FirstPersonGameMode.FirstPersonGameMode_C|GetRngPickupCount _asfirst_person_game_mode_2)
        (:%20%20
          (Variables|Default|SetIsDestroyed true))))
    (:Health
      (bind _asfirst_person_character_3 (Utilities|Casting|CastToFirstPersonCharacter (Game|Player|GetPlayerPawn 0)))
      (bind _output_get (Variables|/Game/FirstPersonBP/Blueprints/FirstPersonCharacter.FirstPersonCharacter_C|SetMaxHealth _asfirst_person_character_3 (+ (Variables|/Game/FirstPersonBP/Blueprints/FirstPersonCharacter.FirstPersonCharacter_C|GetMaxHealth _asfirst_person_character_3) 1e+02)))
      (Variables|/Game/FirstPersonBP/Blueprints/FirstPersonCharacter.FirstPersonCharacter_C|SetHealth _asfirst_person_character_3 _output_get)
      (bind _asfirst_person_game_mode_3 (Utilities|Casting|CastToFirstPersonGameMode (Game|GetGameMode)))
      (Math|Integer|IncrementInt (Variables|/Game/FirstPersonBP/Blueprints/FirstPersonGameMode.FirstPersonGameMode_C|GetHpPickupCount _asfirst_person_game_mode_3)
        (:%20%20
          (Variables|Default|SetIsDestroyed true))))
    (:Speed
      (bind _asfirst_person_character_4 (Utilities|Casting|CastToFirstPersonCharacter (Game|Player|GetPlayerPawn 0)))
      (Variables|/Script/Engine.CharacterMovementComponent|SetMaxWalkSpeed (Actor|GetComponentbyClass _asfirst_person_character_4 "/Script/Engine.CharacterMovementComponent") (+ (Class|MovementComponent|GetMaxSpeed (Actor|GetComponentbyClass _asfirst_person_character_4 "/Script/Engine.CharacterMovementComponent")) 1.5e+02))
      (bind _asfirst_person_game_mode_4 (Utilities|Casting|CastToFirstPersonGameMode (Game|GetGameMode)))
      (Math|Integer|IncrementInt (Variables|/Game/FirstPersonBP/Blueprints/FirstPersonGameMode.FirstPersonGameMode_C|GetSpdPickupCount _asfirst_person_game_mode_4)
        (:%20%20
          (Variables|Default|SetIsDestroyed true))))))