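; BP_Chaser is the Chaser variant of an AI character, configuring its stats on spawn and leaving other behavior to its parent class.
; On BeginPlay it sets its type, scales max health linearly with the floor index from FirstPersonGameMode, and assigns fixed damage and mesh scale.
; A failed game mode cast skips everything after the type assignment.
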(event EventBeginPlay
  (|CallParentFunction)
  (Variables|Default|SetType "Chaser")
  (bind _asfirst_person_game_mode (Utilities|Casting|CastToFirstPersonGameMode (Game|GetGameMode)))
  (Variables|Default|SetMaxHealth (Math|Conversions|ToFloat(Integer) (* (Variables|/Game/FirstPersonBP/Blueprints/FirstPersonGameMode.FirstPersonGameMode_C|GetFloorIndex _asfirst_person_game_mode) 100)))
  (Variables|Default|SetDamage 50)
  (Transformation|SetWorldScale3D (Variables|Character|GetMesh) "1.000000,1.000000,1.000000"))

(event Collision|EventActorBeginOverlap
  (params (OtherActor :type Actor%20Object%20Reference))
  (|CallParentFunction OtherActor) ; This node is disabled and will not be called.\nDrag off pins to build functionality.
)

(event EventTick
  (params (DeltaSeconds :type Float%20%28single-precision%29))
  (|CallParentFunction DeltaSeconds) ; This node is disabled and will not be called.\nDrag off pins to build functionality.
)

(fn ConstructionScript
  (|CallParentFunction))