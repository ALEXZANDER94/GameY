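; AI controller for Chaser, Spitter and Brute enemies that feeds blackboard keys for their behavior logic.
; Once the enemy's AI has started, Tick writes the player's location and runs a distance check per enemy type.
; Chasers and Brutes attack up close, with Brutes also tracking rush state; Spitters attack from afar, otherwise picking random axis-aligned retreat points scaled by room bounds.
; KillBehavior stops the brain logic.
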(event EventBeginPlay
  (bind _asfirst_person_character (Utilities|Casting|CastToFirstPersonCharacter (Game|Player|GetPlayerPawn 0)))
  (Variables|Default|SetPlayer _asfirst_person_character)
  (bind _asbp_enemy_spawn (Utilities|Casting|CastToBP_EnemySpawn (Variables|Default|GetInstigator)))
  (Variables|Default|SetEnemy _asbp_enemy_spawn))

(event EventTick
  (params (DeltaSeconds :type Float%20%28single-precision%29))
  (bind _asbp_enemy_spawn (Utilities|Casting|CastToBP_EnemySpawn (Variables|Default|GetInstigator)))
  (if (Variables|/Game/BP_EnemySpawn.BP_EnemySpawn_C|GetAIBehaviorStarted _asbp_enemy_spawn)
    (AI|Components|Blackboard|SetValueasVector (AI|GetBlackboard 0) (Utilities|Name|MakeLiteralName "PlayerLocation") (Transformation|GetActorLocation (Variables|Default|GetPlayer)))
    (switch Utilities|FlowControl|Switch|SwitchonEnemyType (Variables|/Script/GameY.EnemySpawn|GetType (Variables|Default|GetEnemy))
      (:Chaser
        (CallFunction|ChaserAIBehavior))
      (:Spitter
        (CallFunction|SpitterAIBehavior))
      (:Brute
        (CallFunction|BruteAIBehavior)))))

(fn ConstructionScript)

(fn DistancetoPlayer
  (return (Math|Vector|Distance(Vector) (Transformation|GetActorLocation (Variables|Default|GetPlayer)) (Transformation|GetActorLocation (Variables|Default|GetEnemy)))))

(fn KillBehavior
  (bind _self self)
  (bind _braincomponent (Variables|Default|GetBrainComponent _self))
  (if (Utilities|IsValid _braincomponent)
    (AI|Logic|StopLogic _braincomponent "")))

(fn SpitterAIBehavior
  (bind _player (Variables|Default|GetPlayer))
  (bind _enemy (Variables|Default|GetEnemy))
  (bind _returnvalue (Transformation|GetActorLocation _player))
  (bind _room (Variables|/Game/BP_EnemySpawn.BP_EnemySpawn_C|GetRoom _enemy))
  (bind _boxextent (Collision|GetActorBounds _room false false))
  (bind (_x _y _z) (Math|Vector|BreakVector _returnvalue))
  (bind _returnvalue_2 (Math|Random|RandomFloatinRange 6e+02 (.y _boxextent)))
  (bind _returnvalue_3 (Math|Random|RandomFloatinRange 6e+02 (.x _boxextent)))
  (AI|SetFocus (Variables|Default|GetPlayer))
  (if (> (CallFunction|DistancetoPlayer) 5e+02)
    (AI|Components|Blackboard|SetValueasBool (AI|GetBlackboard 0) (Utilities|Name|MakeLiteralName "InAttackRange") true)
    (else
      (AI|ClearFocus)
      (AI|Components|Blackboard|SetValueasBool (AI|GetBlackboard 0) (Utilities|Name|MakeLiteralName "InAttackRange") false)
      (AI|Components|Blackboard|SetValueasVector (AI|GetBlackboard 0) (Utilities|Name|MakeLiteralName "SafeLocation") (Utilities|Select :Index (Math|Random|RandomInteger 4) :Option%200 (Math|Vector|MakeVector (+ _x _returnvalue_3) _y _z) :Option%201 (Math|Vector|MakeVector (- _x _returnvalue_3) _y _z) :Option%202 (Math|Vector|MakeVector _x (+ _y _returnvalue_2) _z) :Option%203 (Math|Vector|MakeVector _x (- _y _returnvalue_2) _z))))))

(fn BruteAIBehavior
  (bind _asbp_brute (Utilities|Casting|CastToBP_Brute (Variables|Default|GetEnemy)))
  (AI|Components|Blackboard|SetValueasBool (AI|GetBlackboard 0) (Utilities|Name|MakeLiteralName "CanRush") (Variables|/Game/AI/Brute/BP_Brute.BP_Brute_C|GetCanRushAgain _asbp_brute))
  (if (and (<= (CallFunction|DistancetoPlayer) 1.6e+02) (not (Variables|/Game/AI/Brute/BP_Brute.BP_Brute_C|GetRushing _asbp_brute)))
    (AI|Components|Blackboard|SetValueasBool (AI|GetBlackboard 0) (Utilities|Name|MakeLiteralName "InAttackRange") true)
    (else
      (AI|Components|Blackboard|SetValueasBool (AI|GetBlackboard 0) (Utilities|Name|MakeLiteralName "InAttackRange") false))))

(fn ChaserAIBehavior
  (if (<= (CallFunction|DistancetoPlayer) 1.6e+02)
    (AI|Components|Blackboard|SetValueasBool (AI|GetBlackboard 0) (Utilities|Name|MakeLiteralName "InAttackRange") true)
    (else
      (AI|Components|Blackboard|SetValueasBool (AI|GetBlackboard 0) (Utilities|Name|MakeLiteralName "InAttackRange") false))))