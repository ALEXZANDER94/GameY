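; BP_Spitter is a ranged AI enemy, built on a parent class, that fires spitter projectiles.
; On BeginPlay it sets its type, scales max health with the game mode's floor index, sets a fixed damage and shrinks its mesh.
; Shoot spawns a projectile at the Sphere component, aimed along the capsule's forward vector, and passes itself to it as the owning Spitter.
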(event EventBeginPlay
  (|CallParentFunction)
  (Variables|Default|SetType "Spitter")
  (bind _asfirst_person_game_mode (Utilities|Casting|CastToFirstPersonGameMode (Game|GetGameMode)))
  (Variables|Default|SetMaxHealth (Math|Conversions|ToFloat(Integer) (* (Variables|/Game/FirstPersonBP/Blueprints/FirstPersonGameMode.FirstPersonGameMode_C|GetFloorIndex _asfirst_person_game_mode) 75)))
  (Variables|Default|SetDamage 75)
  (Transformation|SetWorldScale3D (Variables|Character|GetMesh) "0.750000,0.750000,0.750000"))

(event Collision|EventActorBeginOverlap
  (params (OtherActor :type Actor%20Object%20Reference))
  (|CallParentFunction OtherActor) ; This node is disabled and will not be called.\nDrag off pins to build functionality.
)

(event EventTick
  (params (DeltaSeconds :type Float%20%28single-precision%29))
  (|CallParentFunction DeltaSeconds) ; This node is disabled and will not be called.\nDrag off pins to build functionality.
)

(fn ConstructionScript
  (|CallParentFunction))

(fn Shoot
  (bind _returnvalue (Game|SpawnActorfromClass "/Game/AI/Spitter/BP_SpitterProjetile.BP_SpitterProjetile_C" (Math|Transform|MakeTransform (Transformation|GetWorldLocation (Variables|Default|GetSphere)) (Math|Conversions|RotationFromXVector (Math|Vector|GetForwardVector (Variables|Default|GetCapsuleComponent self)))) "AlwaysSpawn" 0 0))
  (Variables|/Game/AI/Spitter/BP_SpitterProjetile.BP_SpitterProjetile_C|SetSpitter _returnvalue self))