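; Projectile for the Spitter AI that damages the first-person player and can be destroyed by other projectiles.
; On hit it applies the Spitter's damage to the player and destroys itself, or destroys both actors when the other component is a Projectile.
; Tick extends its lifespan once when the player's LifeSpan value is positive.
; A Damage power-up handler raises its own Damage variable, which the hit logic does not read.
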(event EventBeginPlay)

(event EventTick
  (params (DeltaSeconds :type Float%20%28single-precision%29))
  (bind _asfirst_person_character (Utilities|Casting|CastToFirstPersonCharacter (Game|Player|GetPlayerPawn 0)))
  (if (> (Variables|/Game/FirstPersonBP/Blueprints/FirstPersonCharacter.FirstPersonCharacter_C|GetLifeSpan _asfirst_person_character) 0.0)
    (Utilities|FlowControl|DoOnce false
      (:Completed
        (Actor|SetLifeSpan (+ (Actor|GetLifeSpan) 0.2))))))

(event Collision|EventHit
  (params (MyComp :type Primitive%20Component%20Object%20Reference) (Other :type Actor%20Object%20Reference) (OtherComp :type Primitive%20Component%20Object%20Reference) (bSelfMoved :type Boolean) (HitLocation :type Vector :default "0, 0, 0") (HitNormal :type Vector :default "0, 0, 0") (NormalImpulse :type Vector :default "0, 0, 0") (Hit :type Hit%20Result%20Structure%20%28by%20ref%29))
  (bind _asfirst_person_character (Utilities|Casting|CastToFirstPersonCharacter (Game|Player|GetPlayerPawn 0)))
  ;[1 1 1] collides with player
  (if (== _asfirst_person_character Other)
    (Game|Damage|ApplyDamage _asfirst_person_character (Math|Conversions|ToFloat(Integer) (Variables|/Game/BP_EnemySpawn.BP_EnemySpawn_C|GetDamage (Variables|Default|GetSpitter))) 0 self "/Script/Engine.DamageType")
    (Actor|DestroyActor)
    (else
      ;[1 1 1] Collides with another projectile
      (switch Utilities|FlowControl|Switch|SwitchonECollisionChannel (Collision|GetCollisionObjectType OtherComp)
        (:ECC_GameTraceChannel1
          (Actor|DestroyActor Other)
          (Actor|DestroyActor))))))

(fn ConstructionScript)

(fn HandlePowerUpPickUp
  (params (EffectType :type Byte))
  (switch Utilities|FlowControl|Switch|SwitchonEffectType (Utilities|Enum|ByteToEnumEffectType EffectType)
    (:Damage
      (Variables|Default|SetDamage (+ (Variables|Default|GetDamage) 25.0)))))