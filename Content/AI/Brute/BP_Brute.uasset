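; Brute enemy, a larger AI variant whose health scales with the game mode's floor index and which has a forward rush attack.
; Rush drives a timeline that moves the actor forward with swept steps, ending when it finishes or hits a WorldDynamic component.
; A Delay on Tick re-arms the rush every few seconds once AI behavior has started; the Rush event itself never checks that flag.
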(event Custom|Rush
  (bind _returnvalue (Utilities|Time|GetWorldDeltaSeconds))
  (Variables|Default|SetRushing true)
  (Development|PrintString "Rushing")
  (Timeline|RushingTime PlayFromStart
    (:Update
      (bind _sweephitresult (Transformation|SetActorLocation (+ (* (* (Transformation|GetActorForwardVector) 1.8e+03) _returnvalue) (Transformation|GetActorLocation)) true false))
      (if (Utilities|IsValid (.HitComponent (Collision|BreakHitResult _sweephitresult)))
        (switch Utilities|FlowControl|Switch|SwitchonECollisionChannel (Collision|GetCollisionObjectType (.HitComponent (Collision|BreakHitResult _sweephitresult)))
          (:ECC_WorldDynamic
            (Audio|Components|Audio|Stop (Variables|Default|GetRushingTime))
            (Variables|Default|SetRushing false)
            (Variables|Default|SetCanRushAgain false)))))
    (:Finished
      (Variables|Default|SetRushing false)
      (Variables|Default|SetCanRushAgain false))))

(event EventBeginPlay
  (|CallParentFunction)
  (Variables|Default|SetType "Brute")
  (bind _asfirst_person_game_mode (Utilities|Casting|CastToFirstPersonGameMode (Game|GetGameMode)))
  (Variables|Default|SetMaxHealth (Math|Conversions|ToFloat(Integer) (* (Variables|/Game/FirstPersonBP/Blueprints/FirstPersonGameMode.FirstPersonGameMode_C|GetFloorIndex _asfirst_person_game_mode) 175)))
  (Variables|Default|SetDamage 100)
  (Transformation|SetWorldScale3D (Variables|Character|GetMesh) "1.250000,1.250000,1.250000")
  (Variables|Default|SetCanRushAgain false))

(event Collision|EventActorBeginOverlap
  (params (OtherActor :type Actor%20Object%20Reference))
  (|CallParentFunction OtherActor) ; This node is disabled and will not be called.\nDrag off pins to build functionality.
)

(event EventTick
  (params (DeltaSeconds :type Float%20%28single-precision%29))
  (|CallParentFunction DeltaSeconds)
  (if (Variables|Default|GetAIBehaviorStarted)
    (Utilities|FlowControl|Delay 4.0)
    (Variables|Default|SetCanRushAgain true)))

(fn ConstructionScript
  (|CallParentFunction))