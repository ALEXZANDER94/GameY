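; Boss room of a floor, which spawns BP_FloorBoss at its center and re-skins adjoining doors with the boss material.
; When the player first enters the uncleared room, a boss bar appears and a timeline closes doors and lights the room with input disabled, then starts the boss AI.
; OpenHatch animates the next-level hatch open.
; Reaching the EndFloor trigger shows the end-of-floor widget and pauses the game.
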(event Custom|OpenHatch
  (bind _nextlevelhatch (Variables|Default|GetNextLevelHatch))
  (bind (_direction _hatchinterpspeed _hatchrotinterpspeed) (Timeline|OpenNextLevelHatch Play)
    (:Update
      (Transformation|SetRelativeLocationAndRotation _nextlevelhatch (Math|Vector|Lerp(Vector) (Variables|/Script/Engine.SceneComponent|GetRelativeLocation _nextlevelhatch) (Math|Vector|MakeVector -605.0 4e+01 -195.0) (/ _hatchinterpspeed 3.0)) (Math|Rotator|Lerp(Rotator) (Variables|/Script/Engine.SceneComponent|GetRelativeRotation _nextlevelhatch) "-80.000000, 0, 0" (/ _hatchrotinterpspeed 3.0) true) true false))))

(event Custom|PlayerReachedEnd
  (params (OverlappedComponent :type Primitive%20Component%20Object%20Reference) (OtherActor :type Actor%20Object%20Reference) (OtherComp :type Primitive%20Component%20Object%20Reference) (OtherBodyIndex :type Integer) (bFromSweep :type Boolean) (SweepResult :type Hit%20Result%20Structure%20%28by%20ref%29))
  (bind _asfirst_person_character (Utilities|Casting|CastToFirstPersonCharacter (Game|Player|GetPlayerPawn 0)))
  (if (== OtherActor _asfirst_person_character)
    (bind _returnvalue (UserInterface|CreateWidget "/Game/UI/WBP_EndFloor.WBP_EndFloor_C"))
    (UserInterface|Viewport|AddtoViewport _returnvalue 0)
    (Game|SetGamePaused true)))

(event Custom|PlayerEntersBossRoom
  (params (OverlappedComponent :type Primitive%20Component%20Object%20Reference) (OtherActor :type Actor%20Object%20Reference) (OtherComp :type Primitive%20Component%20Object%20Reference) (OtherBodyIndex :type Integer) (bFromSweep :type Boolean) (SweepResult :type Hit%20Result%20Structure%20%28by%20ref%29))
  (bind _asfirst_person_character (Utilities|Casting|CastToFirstPersonCharacter (Game|Player|GetPlayerPawn 0)))
  (Variables|/Game/FirstPersonBP/Blueprints/FirstPersonCharacter.FirstPersonCharacter_C|SetGridLocation _asfirst_person_character (Variables|Default|GetGridLocation))
  (if (and (== OtherActor _asfirst_person_character) (not (Variables|Default|GetRoomCleared)))
    (Variables|Default|SetVisited true)
    (Utilities|FlowControl|Delay 0.4)
    (Input|DisableInput (Game|Player|GetPlayerPawn 0) (Game|GetPlayerController 0))
    (bind _returnvalue (UserInterface|CreateWidget "/Game/UI/WBP_BossBar.WBP_BossBar_C"))
    (UserInterface|Viewport|AddtoViewport _returnvalue 0)
    (bind (_direction _doorcloseinterpolatin _lightinterpolation) (Timeline|BossLightInterpolation Play)
      (:Update
        (CallFunction|CloseDoors _doorcloseinterpolatin)
        (CallFunction|LightUpRoom _lightinterpolation))
      (:Finished
        (Input|EnableInput (Game|Player|GetPlayerPawn 0) (Game|GetPlayerController 0))
        (Variables|Default|SetDoorsClosed true)
        (for _array_element (Collision|GetOverlappingActors (Variables|Default|GetBoxCollider) "/Game/Boss/BP_FloorBoss.BP_FloorBoss_C" :!class /Script/Engine.PrimitiveComponent)
          (bind _asbp_floor_boss (Utilities|Casting|CastToBP_FloorBoss _array_element))
          (Default|StartAIBehavior _asbp_floor_boss))))))

(event EventBeginPlay
  (|CallParentFunction)
  (Collision|AssignOnComponentBeginOverlap (Variables|Default|GetBoxCollider) (delegate Custom|PlayerEntersBossRoom))
  (CallFunction|TurnDoorsSkull)
  (CallFunction|SpawnBoss)
  (Collision|AssignOnComponentBeginOverlap (Variables|Default|GetEndFloor) (delegate Custom|PlayerReachedEnd)))

(event Collision|EventActorBeginOverlap
  (params (OtherActor :type Actor%20Object%20Reference))
  (|CallParentFunction OtherActor) ; This node is disabled and will not be called.\nDrag off pins to build functionality.
)

(event EventTick
  (params (DeltaSeconds :type Float%20%28single-precision%29))
  (|CallParentFunction DeltaSeconds))

(fn ConstructionScript
  (|CallParentFunction))

(fn TurnDoorsSkull
  (bind _self self)
  (for _array_element (Utilities|Array|MakeArray (Variables|/Game/Rooms/BP_Room.BP_Room_C|GetRoomCollider0 _self) (Variables|/Game/Rooms/BP_Room.BP_Room_C|GetRoomCollider1 _self) (Variables|/Game/Rooms/BP_Room.BP_Room_C|GetRoomCollider2 _self) (Variables|/Game/Rooms/BP_Room.BP_Room_C|GetRoomCollider3 _self))
    (bind _outcomponents (Collision|BoxOverlapComponents (.Origin (Collision|GetComponentBounds _array_element)) (.BoxExtent (Collision|GetComponentBounds _array_element)) (Utilities|Array|MakeArray "ObjectTypeQuery2") "/Game/Rooms/BP_Door.BP_Door_C" 0 :!class /Script/Engine.KismetSystemLibrary))
    (for _array_element_2 _outcomponents
      (Rendering|Material|SetMaterial _array_element_2 0 "/Game/GT_Free2020/Materials/MI_BossDoors.MI_BossDoors"))))

(fn SpawnBoss
  (bind _origin (Collision|GetActorBounds false false))
  (bind _returnvalue (Game|SpawnActorfromClass "/Game/Boss/BP_FloorBoss.BP_FloorBoss_C" (Math|Transform|MakeTransform (Math|Vector|MakeVector (.x _origin) (.y _origin) 9e+01) "0, 0, 0" "1,1,1") "Undefined" 0 0))
  (Variables|/Game/Boss/BP_FloorBoss.BP_FloorBoss_C|SetRoom _returnvalue self)
  (Variables|Default|SetEnemies 1)
  (return))