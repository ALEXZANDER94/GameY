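; Dungeon-style room actor that seals the player in on first entry, lights up, starts its enemy spawners' AI and reopens once no enemies remain.
; On first tick, if the game mode's RoomBuilt is set, it records neighbouring rooms via BP_NoDoor overlaps, disables those blockers and caches door positions by component name.
; Timelines drive VInterpTo door movement and wall light fades, with input disabled while closing.
; Entry also updates the player's GridLocation.
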(event Custom|PlayerHasEnteredRoom
  (params (OverlappedComponent :type Primitive%20Component%20Object%20Reference) (OtherActor :type Actor%20Object%20Reference) (OtherComp :type Primitive%20Component%20Object%20Reference) (OtherBodyIndex :type Integer) (bFromSweep :type Boolean) (SweepResult :type Hit%20Result%20Structure%20%28by%20ref%29))
  (bind _asfirst_person_character (Utilities|Casting|CastToFirstPersonCharacter (Game|Player|GetPlayerPawn 0)))
  (Variables|/Game/FirstPersonBP/Blueprints/FirstPersonCharacter.FirstPersonCharacter_C|SetGridLocation _asfirst_person_character (Variables|Default|GetGridLocation))
  (if (Math|Boolean|ANDBoolean (== OtherActor _asfirst_person_character) (not (Variables|Default|GetRoomCleared)) (not (Variables|Default|GetVisited)))
    (Variables|Default|SetVisited true)
    (Utilities|FlowControl|Delay 0.4)
    (Input|DisableInput (Game|Player|GetPlayerPawn 0) (Game|GetPlayerController 0))
    (bind (_direction _doorcloseinterpolatin _lightinterpolation) (Timeline|DoorCloseInterpolation Play)
      (:Update
        (CallFunction|CloseDoors _doorcloseinterpolatin)
        (CallFunction|LightUpRoom _lightinterpolation))
      (:Finished
        (Input|EnableInput (Game|Player|GetPlayerPawn 0) (Game|GetPlayerController 0))
        (Variables|Default|SetDoorsClosed true)
        (Utilities|FlowControl|Delay 0.5)
        (for _array_element (Collision|GetOverlappingActors (Variables|Default|GetBoxCollider) "/Game/BP_EnemySpawn.BP_EnemySpawn_C" :!class /Script/Engine.PrimitiveComponent)
          (bind _asbp_enemy_spawn (Utilities|Casting|CastToBP_EnemySpawn _array_element))
          (Default|StartAIBehavior _asbp_enemy_spawn))))))

(event EventBeginPlay
  (Collision|AssignOnComponentBeginOverlap (Variables|Default|GetBoxCollider) (delegate Custom|PlayerHasEnteredRoom)))

(event Collision|EventActorBeginOverlap
  (params (OtherActor :type Actor%20Object%20Reference)))

(event EventTick
  (params (DeltaSeconds :type Float%20%28single-precision%29))
  (Utilities|FlowControl|Sequence
    (:then_0
      (Utilities|FlowControl|DoOnce false
        (:Completed
          (bind _asfirst_person_game_mode (Utilities|Casting|CastToFirstPersonGameMode (Game|GetGameMode)))
          (if (Variables|/Game/FirstPersonBP/Blueprints/FirstPersonGameMode.FirstPersonGameMode_C|GetRoomBuilt _asfirst_person_game_mode)
            (CallFunction|BuildRoom)
            (CallFunction|SetDoorLocations)))))
    (:then_1
      (Variables|Default|SetRoomCleared (== (Variables|Default|GetEnemies) 0)))
    (:then_2
      (if (and (Variables|Default|GetRoomCleared) (Variables|Default|GetDoorsClosed))
        (bind _dooropen (Timeline|DooropenInterpolation Play)
          (:Update
            (CallFunction|OpenDoors _dooropen)))))))

(fn ConstructionScript)

(fn BuildRoom
  (for _array_element (Utilities|Array|MakeArray (Variables|Default|GetRoomCollider0) (Variables|Default|GetRoomCollider1) (Variables|Default|GetRoomCollider2) (Variables|Default|GetRoomCollider3))
    (bind (_outcomponents _returnvalue) (Collision|BoxOverlapComponents (.Origin (Collision|GetComponentBounds _array_element)) (.BoxExtent (Collision|GetComponentBounds _array_element)) (Utilities|Array|MakeArray "ObjectTypeQuery2") "/Game/Rooms/BP_NoDoor.BP_NoDoor_C" 0 :!class /Script/Engine.KismetSystemLibrary))
    (if _returnvalue
      (for _array_element_2 _outcomponents
        (Utilities|Array|Add (Variables|Default|GetNeighboringRooms) (Components|GetOwner _array_element_2))
        (Rendering|SetVisibility _array_element_2 false false)
        (Collision|SetCollisionEnabled _array_element_2 "NoCollision"))))
  (CallFunction|SetDoorLocations))

(fn OpenDoors
  (params (InterpSpeed :type Float%20%28single-precision%29))
  (for _array_element (Utilities|Array|MakeArray (Variables|Default|GetDoor1_Right) (Variables|Default|GetDoor1_Left) (Variables|Default|GetDoor2_Right) (Variables|Default|GetDoor2_Left) (Variables|Default|GetDoor3_Right) (Variables|Default|GetDoor3_Left) (Variables|Default|GetDoor4_Right) (Variables|Default|GetDoor4_Left))
    (Transformation|SetWorldLocation _array_element (Math|Interpolation|VInterpTo (Transformation|GetWorldLocation _array_element) (.Value (Utilities|Map|Find (Variables|Default|GetDoorOpenedLocations) (Utilities|String|StringToName (Utilities|GetDisplayName _array_element)))) (Utilities|Time|GetWorldDeltaSeconds) InterpSpeed) true false)))

(fn CloseDoors
  (params (InterpSpeed :type Float%20%28single-precision%29))
  (for _array_element (Utilities|Array|MakeArray (Variables|Default|GetDoor1_Right) (Variables|Default|GetDoor1_Left) (Variables|Default|GetDoor2_Right) (Variables|Default|GetDoor2_Left) (Variables|Default|GetDoor3_Right) (Variables|Default|GetDoor3_Left) (Variables|Default|GetDoor4_Right) (Variables|Default|GetDoor4_Left))
    (Transformation|SetWorldLocation _array_element (Math|Interpolation|VInterpTo (Transformation|GetWorldLocation _array_element) (.Value (Utilities|Map|Find (Variables|Default|GetDoorClosedLocations) (Utilities|String|StringToName (Utilities|GetDisplayName _array_element)))) (Utilities|Time|GetWorldDeltaSeconds) InterpSpeed) true false)))

(fn SetDoorLocations
  (Utilities|FlowControl|Sequence
    (:then_0
      (for _array_element (Utilities|Array|MakeArray (Variables|Default|GetDoor1_Right) (Variables|Default|GetDoor1_Left) (Variables|Default|GetDoor2_Right) (Variables|Default|GetDoor2_Left) (Variables|Default|GetDoor3_Right) (Variables|Default|GetDoor3_Left) (Variables|Default|GetDoor4_Right) (Variables|Default|GetDoor4_Left))
        (Utilities|Map|Add (Variables|Default|GetDoorOpenedLocations) (Utilities|String|StringToName (Utilities|GetDisplayName _array_element)) (Transformation|GetWorldLocation _array_element))))
    (:then_1
      (for (_array_element_2 _array_index) (Utilities|Array|MakeArray (Variables|Default|GetDoor1_Right) (Variables|Default|GetDoor1_Left) (Variables|Default|GetDoor2_Left) (Variables|Default|GetDoor2_Right))
        (Utilities|Map|Add (Variables|Default|GetDoorClosedLocations) (Utilities|String|StringToName (Utilities|GetDisplayName _array_element_2)) (- (Transformation|GetWorldLocation _array_element_2) (Math|Vector|SelectVector "-294.500000, 0, 0" "294.500000, 0, 0" (== (Math|Integer|%(Integer) _array_index 2) 0))))))
    (:then_2
      (for (_array_element_3 _array_index_2) (Utilities|Array|MakeArray (Variables|Default|GetDoor3_Right) (Variables|Default|GetDoor3_Left) (Variables|Default|GetDoor4_Left) (Variables|Default|GetDoor4_Right))
        (Utilities|Map|Add (Variables|Default|GetDoorClosedLocations) (Utilities|String|StringToName (Utilities|GetDisplayName _array_element_3)) (- (Transformation|GetWorldLocation _array_element_3) (Math|Vector|SelectVector "0.000000,-294.500000, 0" "0.000000,294.500000, 0" (== (Math|Integer|%(Integer) _array_index_2 2) 0))))))))

(fn LightUpRoom
  (params (LightInterpolation :type Float%20%28single-precision%29))
  (Utilities|FlowControl|Sequence
    (:then_1
      (for _array_element (Utilities|Array|MakeArray (Variables|Default|GetWallLight) (Variables|Default|GetWallLight1) (Variables|Default|GetWallLight2) (Variables|Default|GetWallLight3) (Variables|Default|GetWallLight4) (Variables|Default|GetWallLight5) (Variables|Default|GetWallLight8) (Variables|Default|GetWallLight9) (Variables|Default|GetWallLight10))
        (Rendering|Components|Light|SetIntensity _array_element (Math|Float|Lerp 0.0 8e+03 LightInterpolation))
        (Rendering|SetVisibility _array_element true false)))))