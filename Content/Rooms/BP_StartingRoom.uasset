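; Starting room Blueprint that runs the player's intro sequence on BeginPlay, building on inherited room behavior.
; It copies its grid location to the FirstPersonCharacter and marks itself visited.
; After a short delay it disables player input while the LightInterpolation timeline drives door closing and room lighting.
; When the timeline finishes, it restores input and flags the doors as closed.
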(event EventBeginPlay
  (|CallParentFunction)
  (bind _asfirst_person_character (Utilities|Casting|CastToFirstPersonCharacter (Game|Player|GetPlayerPawn 0)))
  (Variables|/Game/FirstPersonBP/Blueprints/FirstPersonCharacter.FirstPersonCharacter_C|SetGridLocation _asfirst_person_character (Variables|Default|GetGridLocation))
  (Variables|Default|SetVisited true)
  (Utilities|FlowControl|Delay 0.4)
  (Input|DisableInput (Game|Player|GetPlayerPawn 0) (Game|GetPlayerController 0))
  (bind (_direction _doorcloseinterpolatin _lightinterpolation) (Timeline|LightInterpolation Play)
    (:Update
      (CallFunction|CloseDoors _doorcloseinterpolatin)
      (CallFunction|LightUpRoom _lightinterpolation))
    (:Finished
      (Input|EnableInput (Game|Player|GetPlayerPawn 0) (Game|GetPlayerController 0))
      (Variables|Default|SetDoorsClosed true))))

(event Collision|EventActorBeginOverlap
  (params (OtherActor :type Actor%20Object%20Reference))
  (|CallParentFunction OtherActor) ; This node is disabled and will not be called.\nDrag off pins to build functionality.
)

(event EventTick
  (params (DeltaSeconds :type Float%20%28single-precision%29))
  (|CallParentFunction DeltaSeconds) ; This node is disabled and will not be called.\nDrag off pins to build functionality.
)

(fn ConstructionScript
  (|CallParentFunction))