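; Enemy character, apparently the parent of BP_Brute, with Chaser, Spitter and Brute types for a room- and floor-based game.
; Type selects speed, damage, scale, floor-scaled max health and behavior tree through functions not called within this Blueprint.
; Overlapping the player deals fixed contact damage, except a rushing Brute, which uses its Damage value.
; Incoming damage lowers clamped Health; Tick destroys dead enemies and decrements their Room's enemy count.
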(event Custom|OnTakeDamage
  (params (DamagedActor :type Actor%20Object%20Reference) (Damage :type Float%20%28single-precision%29) (DamageType :type Damage%20Type%20Object%20Reference) (InstigatedBy :type Controller%20Object%20Reference) (DamageCauser :type Actor%20Object%20Reference))
  (CallFunction|SubtractHealth Damage))

(event Custom|OverlappedPlayer
  (params (OverlappedActor :type Actor%20Object%20Reference) (OtherActor :type Actor%20Object%20Reference))
  (CallFunction|OverlappedDamage OtherActor OverlappedActor))

(event EventBeginPlay
  (EventDispatchers|AssignOnTakeAnyDamage (delegate Custom|OnTakeDamage))
  (Collision|BindEventtoOnActorBeginOverlap (delegate Custom|OverlappedPlayer)))

(event Collision|EventActorBeginOverlap
  (params (OtherActor :type Actor%20Object%20Reference)))

(event EventTick
  (params (DeltaSeconds :type Float%20%28single-precision%29))
  (bind _room (Variables|Default|GetRoom))
  (if (CallFunction|IsDead)
    (Actor|DestroyActor)
    (Variables|/Game/Rooms/BP_Room.BP_Room_C|SetEnemies _room (- (Variables|/Game/Rooms/BP_Room.BP_Room_C|GetEnemies _room) 1))))

(fn ConstructionScript)

(fn SubtractHealth
  (params (DamageToApply :type Float%20%28single-precision%29))
  (Variables|Default|SetHealth (Math|Float|Clamp(Float) (- (Variables|Default|GetHealth) DamageToApply) 0.0 (Variables|Default|GetMaxHealth)))
  (return))

(fn IsDead
  (return (<= (Variables|Default|GetHealth) 0.0)))

(fn StartAIBehavior
  (switch Utilities|FlowControl|Switch|SwitchonEnemyType (Variables|Default|GetType)
    (:Chaser
      (AI|RunBehaviorTree (AI|GetAIController self) "/Game/AI/Chaser/BT_Chaser.BT_Chaser"))
    (:Spitter
      (AI|RunBehaviorTree (AI|GetAIController self) "/Game/AI/Spitter/BT_Spitter.BT_Spitter"))
    (:Brute
      (AI|RunBehaviorTree (AI|GetAIController self) "/Game/AI/Brute/BT_Brute.BT_Brute")))
  (Variables|Default|SetAIBehaviorStarted true))

(fn SetEnemyAttributes
  (switch Utilities|FlowControl|Switch|SwitchonEnemyType (Variables|Default|GetType)
    (:Chaser
      (Variables|/Script/Engine.CharacterMovementComponent|SetMaxWalkSpeed (Variables|Character|GetCharacterMovement) 5e+02)
      (bind _asfirst_person_game_mode (Utilities|Casting|CastToFirstPersonGameMode (Game|GetGameMode)))
      (Variables|Default|SetMaxHealth (Math|Conversions|ToFloat(Integer) (* (Variables|/Game/FirstPersonBP/Blueprints/FirstPersonGameMode.FirstPersonGameMode_C|GetFloorIndex _asfirst_person_game_mode) 100)))
      (Variables|Default|SetDamage 50)
      (Transformation|SetWorldScale3D (Variables|Character|GetMesh) "1.000000,1.000000,1.000000"))
    (:Spitter
      (Variables|/Script/Engine.CharacterMovementComponent|SetMaxWalkSpeed (Variables|Character|GetCharacterMovement) 8e+02)
      (bind _asfirst_person_game_mode_2 (Utilities|Casting|CastToFirstPersonGameMode (Game|GetGameMode)))
      (Variables|Default|SetMaxHealth (Math|Conversions|ToFloat(Integer) (* (Variables|/Game/FirstPersonBP/Blueprints/FirstPersonGameMode.FirstPersonGameMode_C|GetFloorIndex _asfirst_person_game_mode_2) 75)))
      (Variables|Default|SetDamage 75)
      (Transformation|SetWorldScale3D (Variables|Character|GetMesh) "0.750000,0.750000,0.750000"))
    (:Brute
      (Variables|/Script/Engine.CharacterMovementComponent|SetMaxWalkSpeed (Variables|Character|GetCharacterMovement) 3e+02)
      (bind _asfirst_person_game_mode_3 (Utilities|Casting|CastToFirstPersonGameMode (Game|GetGameMode)))
      (Variables|Default|SetMaxHealth (Math|Conversions|ToFloat(Integer) (* (Variables|/Game/FirstPersonBP/Blueprints/FirstPersonGameMode.FirstPersonGameMode_C|GetFloorIndex _asfirst_person_game_mode_3) 175)))
      (Variables|Default|SetDamage 100)
      (Transformation|SetWorldScale3D (Variables|Character|GetMesh) "1.250000,1.250000,1.250000"))))

(fn KillBehavior
  (bind _asbp_enemy_aicontroller (Utilities|Casting|CastToBP_EnemyAIController (AI|GetAIController self)))
  (Default|KillBehavior _asbp_enemy_aicontroller))

(fn OverlappedDamage
  (params (B :type Object%20Object%20Reference) (Object :type Object%20Object%20Reference))
  (bind _asfirst_person_character (Utilities|Casting|CastToFirstPersonCharacter (Game|Player|GetPlayerPawn 0)))
  (if (== _asfirst_person_character B)
    (bind _asbp_enemy_spawn (Utilities|Casting|CastToBP_EnemySpawn Object))
    (switch Utilities|FlowControl|Switch|SwitchonEnemyType (Variables|/Script/GameY.EnemySpawn|GetType _asbp_enemy_spawn)
      (:Chaser
        (Game|Damage|ApplyDamage _asfirst_person_character 25.0 0 0 "/Script/Engine.DamageType" :!label _label))
      (:Spitter
        (goto _label))
      (:Brute
        (bind _asbp_brute (Utilities|Casting|CastToBP_Brute _asbp_enemy_spawn))
        (if (Variables|/Game/AI/Brute/BP_Brute.BP_Brute_C|GetRushing _asbp_brute)
          (Game|Damage|ApplyDamage _asfirst_person_character (Math|Conversions|ToFloat(Integer) (Variables|BP_EnemySpawn_C|GetDamage _asbp_brute)) 0 _asbp_brute "/Script/Engine.DamageType")
          (else
            (Game|Damage|ApplyDamage _asfirst_person_character 25.0 0 _asbp_brute "/Script/Engine.DamageType")))))))