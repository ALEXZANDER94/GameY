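; Floor boss character whose max health scales with the game mode's floor index and whose death opens its room's hatch.
; StartAIBehavior runs BT_Boss; attack functions toggle ABP_Boss flags, reset by timers, and IsPlayerHit tests 2D range, offset forward when RushFlag is set.
; Damage events reduce health, overlapping the player deals damage, and Tick destroys the boss at zero health or re-arms RushFlag through a delay and timer.
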(event Custom|OnTakeDamage
  (params (DamagedActor :type Actor%20Object%20Reference) (Damage :type Float%20%28single-precision%29) (DamageType :type Damage%20Type%20Object%20Reference) (InstigatedBy :type Controller%20Object%20Reference) (DamageCauser :type Actor%20Object%20Reference))
  (CallFunction|SubtractHealth Damage))

(event Custom|OverlappedPlayer
  (params (OverlappedActor :type Actor%20Object%20Reference) (OtherActor :type Actor%20Object%20Reference))
  (CallFunction|OverlappedDamage OtherActor OverlappedActor))

(event Custom|BossIsDead
  (params (DestroyedActor :type Actor%20Object%20Reference))
  (bind _asbp_boss_room (Utilities|Casting|CastToBP_BossRoom (Variables|Default|GetRoom)))
  (Default|OpenHatch _asbp_boss_room))

(event EventBeginPlay
  (CallFunction|SetVariables)
  (EventDispatchers|AssignOnTakeAnyDamage (delegate Custom|OnTakeDamage))
  (EventDispatchers|AssignOnActorBeginOverlap (delegate Custom|OverlappedPlayer))
  (Game|AssignOnDestroyed (delegate Custom|BossIsDead)))

(event Collision|EventActorBeginOverlap
  (params (OtherActor :type Actor%20Object%20Reference)))

(event EventTick
  (params (DeltaSeconds :type Float%20%28single-precision%29))
  (if (CallFunction|IsDead)
    (Actor|DestroyActor)
    (else
      (Utilities|FlowControl|Sequence
        (:then_0
          (if (and (Variables|Default|GetAIBehaviorStarted) (not (Variables|Default|GetRushFlag)))
            (Utilities|Time|SetTimerbyFunctionName 0 "StartRushAgain" 6.0)))
        (:then_1
          (if (not (Math|Boolean|NANDBoolean (not (Variables|Default|GetRushFlag)) (Variables|Default|GetAIBehaviorStarted)))
            (Utilities|FlowControl|Delay 6.0)
            (Variables|Default|SetRushFlag true)
            (Development|PrintString "Able to Rush Again")))))))

(fn ConstructionScript)

(fn SubtractHealth
  (params (DamageToApply :type Float%20%28single-precision%29))
  (Variables|Default|SetHealth (Math|Float|Clamp(Float) (- (Variables|Default|GetHealth) DamageToApply) 0.0 (Variables|Default|GetMaxHealth)))
  (return))

(fn OverlappedDamage
  (params (B :type Object%20Object%20Reference) (Object :type Object%20Object%20Reference))
  (bind _asfirst_person_character (Utilities|Casting|CastToFirstPersonCharacter (Game|Player|GetPlayerPawn 0)))
  (if (== _asfirst_person_character B)
    (Game|Damage|ApplyDamage _asfirst_person_character 5e+01 0 0 "/Script/Engine.DamageType")))

(fn IsDead
  (return (<= (Variables|Default|GetHealth) 0.0)))

(fn SetVariables
  (Variables|Default|SetBossName "Generic Boss")
  (bind _asfirst_person_game_mode (Utilities|Casting|CastToFirstPersonGameMode (Game|GetGameMode)))
  (Variables|Default|SetMaxHealth (Math|Conversions|ToFloat(Integer) (* (Variables|/Game/FirstPersonBP/Blueprints/FirstPersonGameMode.FirstPersonGameMode_C|GetFloorIndex _asfirst_person_game_mode) 300))))

(fn StartAIBehavior
  (AI|RunBehaviorTree (AI|GetAIController self) "/Game/Boss/BT_Boss.BT_Boss")
  (Variables|Default|SetAIBehaviorStarted true))

(fn Attack
  (bind _asabp_boss (Utilities|Casting|CastToABP_Boss (Components|SkeletalMesh|GetAnimInstance (Variables|Character|GetMesh))))
  (Variables|/Game/Boss/ABP_Boss.ABP_Boss_C|SetAttacking _asabp_boss true)
  (Utilities|Time|SetTimerbyFunctionName 0 "DisableAttacking" 2.0)
  (return))

(fn DisableAttacking
  (bind _asabp_boss (Utilities|Casting|CastToABP_Boss (Components|SkeletalMesh|GetAnimInstance (Variables|Character|GetMesh))))
  (Variables|/Game/Boss/ABP_Boss.ABP_Boss_C|SetAttacking _asabp_boss false)
  (Variables|/Game/Boss/ABP_Boss.ABP_Boss_C|SetRushingAttack _asabp_boss false)
  (Variables|Default|SetRushFlag false)
  (return))

(fn IsPlayerHit
  (bind _asfirst_person_character (Utilities|Casting|CastToFirstPersonCharacter (Game|Player|GetPlayerPawn 0)))
  (if (Variables|Default|GetRushFlag)
    (return (< (Math|Vector|Distance2D(Vector) (Transformation|GetActorLocation _asfirst_person_character) (+ (Transformation|GetActorLocation) (* (Math|Vector|GetForwardVector (Variables|Default|GetCapsuleComponent)) 335))) 2.5e+02))
    (else
      (return (< (Math|Vector|Distance2D(Vector) (Transformation|GetActorLocation _asfirst_person_character) (Transformation|GetActorLocation)) 2.5e+02)))))

(fn RushAttack
  (bind _asabp_boss (Utilities|Casting|CastToABP_Boss (Components|SkeletalMesh|GetAnimInstance (Variables|Character|GetMesh))))
  (Variables|/Game/Boss/ABP_Boss.ABP_Boss_C|SetRushingAttack _asabp_boss true)
  (Utilities|Time|SetTimerbyFunctionName 0 "DisableAttacking" 3.0)
  (return))

(fn StartRushAgain
  (Variables|Default|SetRushFlag true))