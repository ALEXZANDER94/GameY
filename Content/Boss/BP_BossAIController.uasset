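; AI controller for the floor boss that feeds its blackboard with data about the first-person player.
; BeginPlay caches player and boss; once the boss's AI behavior has started, Tick writes the player's location and runs BossBehavior.
; BossBehavior sets InAttackRange when the player is close and the boss isn't attacking.
; Otherwise, the boss's RushFlag either sets RushAgain or clears both flags.
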(event EventBeginPlay
  (bind _asfirst_person_character (Utilities|Casting|CastToFirstPersonCharacter (Game|Player|GetPlayerPawn 0)))
  (Variables|Default|SetPlayer _asfirst_person_character)
  (bind _asbp_floor_boss (Utilities|Casting|CastToBP_FloorBoss (Game|GetInstigator)))
  (Variables|Default|SetBoss _asbp_floor_boss))

(event EventTick
  (params (DeltaSeconds :type Float%20%28single-precision%29))
  (bind _asbp_floor_boss (Utilities|Casting|CastToBP_FloorBoss (Game|GetInstigator)))
  (if (Variables|/Game/Boss/BP_FloorBoss.BP_FloorBoss_C|GetAIBehaviorStarted _asbp_floor_boss)
    (AI|Components|Blackboard|SetValueasVector (AI|GetBlackboard 0) (Utilities|Name|MakeLiteralName "PlayerLocation") (Transformation|GetActorLocation (Variables|Default|GetPlayer)))
    (CallFunction|BossBehavior)))

(fn ConstructionScript)

(fn DistancetoPlayer
  (return (Math|Vector|Distance(Vector) (Transformation|GetActorLocation (Variables|Default|GetPlayer)) (Transformation|GetActorLocation (Variables|Default|GetBoss)))))

(fn BossBehavior
  (if (and (<= (CallFunction|DistancetoPlayer) 1.6e+02) (not (Variables|/Game/Boss/BP_FloorBoss.BP_FloorBoss_C|GetAttacking (Variables|Default|GetBoss))))
    (AI|Components|Blackboard|SetValueasBool (AI|GetBlackboard 0) (Utilities|Name|MakeLiteralName "InAttackRange") true)
    (else
      (switch int (Math|Conversions|ToInteger(Boolean) (Variables|/Game/Boss/BP_FloorBoss.BP_FloorBoss_C|GetRushFlag (Variables|Default|GetBoss)))
        (:0
          (AI|Components|Blackboard|SetValueasBool (AI|GetBlackboard 0) (Utilities|Name|MakeLiteralName "InAttackRange") false)
          (AI|Components|Blackboard|SetValueasBool (AI|GetBlackboard 0) (Utilities|Name|MakeLiteralName "RushAgain") false))
        (:1
          (AI|Components|Blackboard|SetValueasBool (AI|GetBlackboard 0) (Utilities|Name|MakeLiteralName "RushAgain") true))))))